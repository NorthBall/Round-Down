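; AI actor Blueprint that initializes its health and displays it on a widget health bar.
; On BeginPlay it sets a MaxHealth base entry, resets and refreshes stats, sets Health and prints both health values for debugging.
; It then casts the widget component's user widget to HealthBar and sets its health percentage.
; The UpdateHealthBar event re-runs that same bar update on demand.
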(event EventBeginPlay
  (Utilities|Map|Add (Variables|Default|GetBaseA) "MaxHealth" 1000)
  (Class|CommonAncestor|ResetStats)
  (Class|CommonAncestor|UpdateAll)
  (Variables|Default|SetHealth 1000)
  (Development|PrintString (Utilities|String|ToString(Integer) (Variables|Default|GetHealth)))
  (Development|PrintString (Utilities|String|ToString(Integer) (Variables|Default|GetMaxHealth)) true true "(R=0.028321,G=1.000000,B=0.000000,A=1.000000)")
  (bind _ashealth_bar (Utilities|Casting|CastToHealthBar (UserInterface|GetUserWidgetObject (Variables|Default|GetWidget))))
  (Variables|/Game/Widgets/HealthBar.HealthBar_C|SetPercentHealth _ashealth_bar (/ (Math|Conversions|ToFloat(Integer) (Variables|Default|GetHealth)) (Math|Conversions|ToFloat(Integer) (Variables|Default|GetMaxHealth)))))

(event Collision|EventActorBeginOverlap
  (params (OtherActor :type Actor%20Object%20Reference)))

(event EventUpdateHealthBar
  (bind _ashealth_bar (Utilities|Casting|CastToHealthBar (UserInterface|GetUserWidgetObject (Variables|Default|GetWidget))))
  (Variables|/Game/Widgets/HealthBar.HealthBar_C|SetPercentHealth _ashealth_bar (/ (Math|Conversions|ToFloat(Integer) (Variables|Default|GetHealth)) (Math|Conversions|ToFloat(Integer) (Variables|Default|GetMaxHealth)))))

(event EventTick
  (params (DeltaSeconds :type Float%20%28single-precision%29)))

(fn ConstructionScript)